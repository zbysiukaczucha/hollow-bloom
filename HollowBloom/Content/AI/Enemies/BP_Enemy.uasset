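; Enemy character with sword attack montages, a stats-driven health bar, and save/restore of its state, including transform, health and death.
; A looping timer runs sphere traces along the sword (boss uses separate positions) with DoOnce-throttled damage, alongside a single-point attack trace.
; Overlap volumes toggle the health bar and optionally report player range to BP_AI_Enemy.
; Death notifies the AI, ragdolls body and sword, clears player target lock and awards XP.
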(event `self.ReceiveBeginPlay`
  (bind _aswb_enemy_healthbar (cast `/Game/UI/Blueprints/WB_EnemyHealthbar` (`WidgetComponent.GetWidget` (`self.Widget`))))
  (set `/Game/UI/Blueprints/WB_EnemyHealthbar.Stats` (`self.Stats`) _aswb_enemy_healthbar)
  (set `/Game/UI/Blueprints/WB_EnemyHealthbar.EnemyName` (`self.EnemyName`) _aswb_enemy_healthbar)
  (if (== (`self.InitialPosition`) (0.0 0.0 0.0))
    (set `self.InitialPosition` (`self.K2_GetActorLocation`))
    (set `self.InitialRotation` (`self.K2_GetActorRotation`))))

(event `/Game/Blueprints/BPI_Damage.EndSwordTrace`
  ;[1 1 1] Damage trace
  (if (`KismetSystemLibrary.K2_IsValidTimerHandle` (stale `/Game/Blueprints/BPI_Damage.BeginSwordTrace` _returnvalue))
    (`KismetSystemLibrary.K2_ClearAndInvalidateTimerHandle` (stale `/Game/Blueprints/BPI_Damage.BeginSwordTrace` _returnvalue))))

(event `/Game/Blueprints/BPI_Damage.BeginSwordTrace`
  ;[1 1 1] Damage trace
  (bind _returnvalue (`KismetSystemLibrary.K2_SetTimerDelegate` (delegate `DamageTrace`) 0.01 true)))

(event `DamageTrace`
  (bind _isboss (`self.IsBoss`))
  ;[1 1 1] Damage trace
  (bind (_outhit _returnvalue) (`KismetSystemLibrary.SphereTraceSingleForObjects` :`Start` (`KismetMathLibrary.SelectVector` (`self.StartTracePosition`) (`SceneComponent.K2_GetComponentLocation` (`self.Start Sword Trace`)) _isboss) :`End` (`KismetMathLibrary.SelectVector` (`self.EndTracePosition`) (`SceneComponent.K2_GetComponentLocation` (`self.End Sword Trace`)) _isboss) :`Radius` (`self.TraceRadius`) :`ObjectTypes` (`|MakeArray` "ObjectTypeQuery3" :!type "EObjectTypeQuery Enum") :`DrawDebugType` "ForOneFrame"))
  (if _returnvalue
    (`/Engine/EditorBlueprintResources/StandardMacros.DoOnce` false :!label _label
      (:`Completed`
        (`GameplayStatics.ApplyDamage` (`.HitActor` (`GameplayStatics.BreakHitResult` _outhit)) (`self.Sword Damage`))
        (`KismetSystemLibrary.Delay` 0.3)
        (goto _label :!via `Reset`)))))

(event `self.ReceiveAnyDamage`
  (params (Damage :type "Float (single-precision)") (DamageType :type "DamageType Object Reference") (InstigatedBy :type "Controller Object Reference") (DamageCauser :type "Actor Object Reference"))
  (bind _returnvalue (`StatsComponent.DecreaseHealth` (`self.Stats`) Damage))
  (if _returnvalue
    (`self.Die`)))

(event `/Game/Blueprints/BPI_Damage.Die`
  (bind _sword (`self.Sword`))
  (`SceneComponent.K2_DetachFromComponent` _sword "KeepWorld" "KeepWorld" "KeepWorld" false)
  (`PrimitiveComponent.SetCollisionEnabled` _sword "QueryAndPhysics")
  (`PrimitiveComponent.SetSimulatePhysics` _sword true)
  (bind _asbp_ai_enemy (cast `/Game/AI/Enemies/BP_AI_Enemy` (`self.GetController`)))
  (`/Game/AI/Enemies/BP_AI_Enemy.Died` _asbp_ai_enemy)
  (`PrimitiveComponent.SetSimulatePhysics` (`self.Mesh`) true)
  (`ActorComponent.K2_DestroyComponent` (`self.Widget`))
  (`PrimitiveComponent.SetCollisionEnabled` (`self.CapsuleComponent`) "NoCollision")
  (bind _asbp_third_person_character (cast `/Game/ThirdPerson/Blueprints/BP_ThirdPersonCharacter` (`GameplayStatics.GetPlayerCharacter` 0)))
  (bind _combatcomponent (`/Game/ThirdPerson/Blueprints/BP_ThirdPersonCharacter.CombatComponent` _asbp_third_person_character))
  (set `CombatComponent.TargetLockActor` null _combatcomponent)
  (bind _targetlockwidget (`CombatComponent.TargetLockWidget` _combatcomponent)
    (:`then`
      (`self.K2_DestroyActor` _targetlockwidget))
    (:`else`
      _))
  (bind _asbp_third_person_character_2 (cast `/Game/ThirdPerson/Blueprints/BP_ThirdPersonCharacter` (`GameplayStatics.GetPlayerCharacter` 0)))
  (bind _charactermovement (`Character.CharacterMovement` _asbp_third_person_character_2))
  (set `CharacterMovementComponent.bOrientRotationToMovement` true _charactermovement)
  (set `CharacterMovementComponent.bUseControllerDesiredRotation` false _charactermovement)
  (`StatsComponent.IncreaseXP` (`/Game/ThirdPerson/Blueprints/BP_ThirdPersonCharacter.PlayerStats` _asbp_third_person_character_2) (`self.XP_Reward`))
  (set `self.IsDead` true)
  (`self.SetActorTickEnabled` false)
  (`PrimitiveComponent.SetCollisionObjectType` (`self.Mesh`) "ECC_WorldStatic"))

(event `/Game/Blueprints/BPI_Damage.PointDamageTrace`
  (bind _returnvalue (`SceneComponent.K2_GetComponentLocation` (`self.PointTracePos`)))
  (bind (_outhit _returnvalue_2) (`KismetSystemLibrary.SphereTraceSingleForObjects` :`Start` _returnvalue :`End` _returnvalue :`Radius` (`self.PointAttackRadius`) :`ObjectTypes` (`|MakeArray` "ObjectTypeQuery3" :!type "EObjectTypeQuery Enum") :`DrawDebugType` "ForDuration" :`DrawTime` 1.0))
  (if _returnvalue_2
    (`GameplayStatics.ApplyDamage` (`.HitActor` (`GameplayStatics.BreakHitResult` _outhit)) 30.0)))

(event `self.Healthbar Radius.OnComponentBeginOverlap`
  (params (OverlappedComponent :type "PrimitiveComponent Object Reference") (OtherActor :type "Actor Object Reference") (OtherComp :type "PrimitiveComponent Object Reference") (OtherBodyIndex :type Integer) (bFromSweep :type Boolean) (SweepResult :type "HitResult Structure (by ref)"))
  ;[1 1 1] Show health bar
  (cast `/Game/ThirdPerson/Blueprints/BP_ThirdPersonCharacter` OtherActor)
  (bind _widget (`self.Widget`)
    (:`then`
      (`SceneComponent.SetVisibility` _widget true false))
    (:`else`)))

(event `self.Healthbar Radius.OnComponentEndOverlap`
  (params (OverlappedComponent :type "PrimitiveComponent Object Reference") (OtherActor :type "Actor Object Reference") (OtherComp :type "PrimitiveComponent Object Reference") (OtherBodyIndex :type Integer))
  ;[1 1 1] Show health bar
  (cast `/Game/ThirdPerson/Blueprints/BP_ThirdPersonCharacter` OtherActor)
  (bind _widget (`self.Widget`)
    (:`then`
      (`SceneComponent.SetVisibility` _widget false false))
    (:`else`)))

(event `self.ChaseRadius.OnComponentBeginOverlap`
  (params (OverlappedComponent :type "PrimitiveComponent Object Reference") (OtherActor :type "Actor Object Reference") (OtherComp :type "PrimitiveComponent Object Reference") (OtherBodyIndex :type Integer) (bFromSweep :type Boolean) (SweepResult :type "HitResult Structure (by ref)"))
  (if (`self.ChaseInRangeOnly`)
    (cast `/Game/ThirdPerson/Blueprints/BP_ThirdPersonCharacter` OtherActor)
    (bind _asbp_ai_enemy (cast `/Game/AI/Enemies/BP_AI_Enemy` (`self.GetController`)))
    (set `/Game/AI/Enemies/BP_AI_Enemy.PlayerInRange` true _asbp_ai_enemy)))

(event `self.ChaseRadius.OnComponentEndOverlap`
  (params (OverlappedComponent :type "PrimitiveComponent Object Reference") (OtherActor :type "Actor Object Reference") (OtherComp :type "PrimitiveComponent Object Reference") (OtherBodyIndex :type Integer))
  (if (`self.ChaseInRangeOnly`)
    (cast `/Game/ThirdPerson/Blueprints/BP_ThirdPersonCharacter` OtherActor)
    (bind _asbp_ai_enemy (cast `/Game/AI/Enemies/BP_AI_Enemy` (`self.GetController`)))
    (set `/Game/AI/Enemies/BP_AI_Enemy.PlayerInRange` false _asbp_ai_enemy)
    (`/Game/AI/Enemies/BP_AI_Enemy.PlayerLeftRange` _asbp_ai_enemy)))

(fn `GetEnemySave`
  (returns (EnemySave :type "/Game/SaveGame/S_EnemySave Structure"))
  (return (make `/Game/SaveGame/S_EnemySave` (`self.EnemyID`) (`self.GetTransform`) (`StatsComponent.CurrentHealth` (`self.Stats`)) (`self.InitialPosition`) (`self.InitialRotation`) (`self.IsDead`) (`self.IsBoss`))))

(fn `Strong Attack`
  (returns (Duration :type "Float (double-precision)"))
  (bind _returnvalue (`self.PlayAnimMontage` (`self.StrongAttackMontage`)))
  (return _returnvalue))

(fn `SwordAttack`
  (returns (Duration :type "Float (double-precision)"))
  (bind _returnvalue (`self.PlayAnimMontage` (`self.SwordAttackMontage`)))
  (return _returnvalue))

(fn `UseEnemySave`
  (params (EnemySave :type "/Game/SaveGame/S_EnemySave Structure"))
  (`self.K2_SetActorTransform` EnemySave_Transform_2_62EC432C42F26BFED380158A4B5BB29E)
  (set `StatsComponent.CurrentHealth` EnemySave_CurrentHealth_5_FA5798AD498E11D2178252BC6AFDCC78 (`self.Stats`))
  (set `self.IsDead` EnemySave_IsDead_10_66280F0C4CAF1E98AFF674BCB27DB1FD)
  (set `self.InitialPosition` EnemySave_InitialPosition_18_551FFEA9496FDAEDC2001784974E26DD)
  (set `self.InitialRotation` EnemySave_InitialRotation_19_C65C623540E89276256DCE94CC7F62F2))

(fn `UserConstructionScript`)