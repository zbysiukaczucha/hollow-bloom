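; BP_NPC is a roaming, talkable NPC driven by a DialogueComponent and a data table.
; It repeatedly moves to random reachable points, and shows a "Talk" widget while the player character is inside its interact radius.
; Interacting begins dialogue and disables movement until the end-dialogue event restores walking.
; On BeginPlay it restores any saved dialogue row from the GameInstance, and exposes the current row for saving.
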(event `self.ReceiveBeginPlay`
  ;[1 1 1] Set up npc movement
  (`self.RandomRoam`)
  (add `/Game/Dialogue/DialogueComponent.EndDialogueEvent` (`self.DialogueComponent`) (delegate `EndDialogue`))
  ;[1 1 1] Set interaction text
  (bind _aswb_interact (cast `/Game/UI/Blueprints/WB_Interact` (`WidgetComponent.GetWidget` (`self.Interact Widget`))))
  (set `/Game/UI/Blueprints/WB_Interact. Text` "Talk" _aswb_interact)
  (bind _output_get (set `/Game/Dialogue/DialogueComponent.Data Table` (`self.Dialogue Data Table`) (`self.DialogueComponent`)))
  (bind _savegamedata (message `/Game/SaveGame/BPI_SaveGame.GetGameData` (`GameplayStatics.GetGameInstance`)))
  (bind (_value _returnvalue) (`BlueprintMapLibrary.Map_Find` (`/Game/SaveGame/BP_Save.DialogueRows` _savegamedata) _output_get))
  (if _returnvalue
    (`self.UseDialogueSave` _value)))

(event `EndDialogue`
  ;[1 1 1] Set up npc movement
  (`CharacterMovementComponent.SetMovementMode` (`self.CharacterMovement`) "MOVE_Walking" 0))

(event `self.Interact radius.OnComponentBeginOverlap`
  (params (OverlappedComponent :type "PrimitiveComponent Object Reference") (OtherActor :type "Actor Object Reference") (OtherComp :type "PrimitiveComponent Object Reference") (OtherBodyIndex :type Integer) (bFromSweep :type Boolean) (SweepResult :type "HitResult Structure (by ref)"))
  ;[1 1 1] Interact prompt visibility
  (cast `/Game/ThirdPerson/Blueprints/BP_ThirdPersonCharacter` OtherActor)
  (`SceneComponent.SetVisibility` (`self.Interact Widget`) true false))

(event `self.Interact radius.OnComponentEndOverlap`
  (params (OverlappedComponent :type "PrimitiveComponent Object Reference") (OtherActor :type "Actor Object Reference") (OtherComp :type "PrimitiveComponent Object Reference") (OtherBodyIndex :type Integer))
  ;[1 1 1] Interact prompt visibility
  (cast `/Game/ThirdPerson/Blueprints/BP_ThirdPersonCharacter` OtherActor)
  (`SceneComponent.SetVisibility` (`self.Interact Widget`) false false))

(event `self.OnInteract`
  (params (Interactor :type "Actor Object Reference"))
  ;[1 1 1] Interaction
  (`/Game/Dialogue/DialogueComponent.BeginDialogue` (`self.DialogueComponent`))
  (`CharacterMovementComponent.DisableMovement` (`self.CharacterMovement`)))

(event `RandomRoam`
  ;[1 1 1] Idle movement
  (`|AIMoveTo` self (`NavigationSystemV1.K2_GetRandomReachablePointInRadius` (`self.K2_GetActorLocation`) 2000.0 null null) null
    (:`OnSuccess`
      (`KismetSystemLibrary.Delay` 1.0)
      (`self.RandomRoam`))))

(fn `GetDialogueSave`
  (returns (RowName :type Name))
  (return (`/Game/Dialogue/DialogueComponent.Row Name` (`self.DialogueComponent`))))

(fn `UseDialogueSave`
  (params (RowName :type Name))
  (set `/Game/Dialogue/DialogueComponent.Row Name` RowName (`self.DialogueComponent`)))

(fn `UserConstructionScript`)