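; BP_QuestItem_Child is a quest item, derived from a parent Blueprint, that reacts to a successful roll.
; On Roll Success swaps both static mesh material slots to rotation materials.
; It then casts the player to BP_ThirdPersonCharacter, starts and immediately completes quest "1" on its QuestComponent, and hides the interact widget.
; The event graph holds only disabled default nodes.
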(fn `On Roll Success`
  (bind _staticmesh (`self.StaticMesh`))
  (`PrimitiveComponent.SetMaterial` _staticmesh 0 "/Game/Medieval_Env/Props/Materials/MI_RotationWood.MI_RotationWood")
  (`PrimitiveComponent.SetMaterial` _staticmesh 1 "/Game/Medieval_Env/Props/Materials/M_Master_Rotation.M_Master_Rotation")
  (bind _asbp_third_person_character (cast `/Game/ThirdPerson/Blueprints/BP_ThirdPersonCharacter` (`GameplayStatics.GetPlayerCharacter` 0)))
  (bind _questcomponent (`/Game/ThirdPerson/Blueprints/BP_ThirdPersonCharacter.QuestComponent` _asbp_third_person_character))
  (`/Game/Quests/QuestComponent.StartQuest` _questcomponent "1")
  (`/Game/Quests/QuestComponent.CompleteQuest` _questcomponent "1")
  (`SceneComponent.SetVisibility` (`self.InteractWidget`) false false))

(fn `UserConstructionScript`
  (`parent.UserConstructionScript`))