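; BP_LogPile is a log pile actor that changes its appearance when the roll inherited from its parent class succeeds.
; On Roll Success runs the parent logic, hides StaticMesh with its children, and turns off collision on it and its child mesh components.
; It then swaps the StackedPile mesh to SM_LogPile_04.
; BeginPlay and the construction script only call the parent.
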(event `self.ReceiveBeginPlay`
  (`parent.ReceiveBeginPlay`))

(fn `On Roll Success`
  (bind _staticmesh (`self.StaticMesh`))
  (`parent.On Roll Success`)
  (`SceneComponent.SetVisibility` _staticmesh false true)
  (`PrimitiveComponent.SetCollisionEnabled` _staticmesh "NoCollision")
  (for _array_element (`SceneComponent.GetChildrenComponents` _staticmesh true)
    (bind _asstatic_mesh_component (cast `StaticMeshComponent` _array_element))
    (`PrimitiveComponent.SetCollisionEnabled` _asstatic_mesh_component "NoCollision"))
  (`StaticMeshComponent.SetStaticMesh` (`self.StackedPile`) "/Game/Medieval_Village_Props/Meshes/Props/StableProps/SM_LogPile_04.SM_LogPile_04"))

(fn `UserConstructionScript`
  (`parent.UserConstructionScript`))