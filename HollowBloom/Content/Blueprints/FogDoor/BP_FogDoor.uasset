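; BP_FogDoor is an interactable fog wall that lets the player pass through it once.
; Overlapping its box shows a "Traverse the mist" widget while interaction is enabled, and leaving hides it.
; On interact, it disables Layer3 collision, calls MoveForward on the third-person character, then restores collision after a short delay and disables further interaction.
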(event `self.ReceiveBeginPlay`
  (bind _aswb_interact (cast `/Game/UI/Blueprints/WB_Interact` (`WidgetComponent.GetWidget` (`self.Interact Widget`))))
  (set `/Game/UI/Blueprints/WB_Interact. Text` "Traverse \nthe mist" _aswb_interact))

(event `self.OnInteract`
  (params (Interactor :type "Actor Object Reference"))
  (if (`self.EnableInteraction`)
    (`PrimitiveComponent.SetCollisionEnabled` (`self.Layer3`) "NoCollision")
    (bind _asbp_third_person_character (cast `/Game/ThirdPerson/Blueprints/BP_ThirdPersonCharacter` Interactor))
    (`/Game/ThirdPerson/Blueprints/BP_ThirdPersonCharacter.MoveForward` _asbp_third_person_character)
    (`KismetSystemLibrary.Delay` 0.5)
    (`PrimitiveComponent.SetCollisionEnabled` (`self.Layer3`) "QueryAndPhysics")
    (set `self.EnableInteraction` false)))

(event `self.Box.OnComponentBeginOverlap`
  (params (OverlappedComponent :type "PrimitiveComponent Object Reference") (OtherActor :type "Actor Object Reference") (OtherComp :type "PrimitiveComponent Object Reference") (OtherBodyIndex :type Integer) (bFromSweep :type Boolean) (SweepResult :type "HitResult Structure (by ref)"))
  (if (`self.EnableInteraction`)
    (cast `/Game/ThirdPerson/Blueprints/BP_ThirdPersonCharacter` OtherActor)
    (`SceneComponent.SetVisibility` (`self.Interact Widget`) true false)))

(event `self.Box.OnComponentEndOverlap`
  (params (OverlappedComponent :type "PrimitiveComponent Object Reference") (OtherActor :type "Actor Object Reference") (OtherComp :type "PrimitiveComponent Object Reference") (OtherBodyIndex :type Integer))
  (cast `/Game/ThirdPerson/Blueprints/BP_ThirdPersonCharacter` OtherActor)
  (`SceneComponent.SetVisibility` (`self.Interact Widget`) false false))

(fn `UserConstructionScript`)