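; BP_QuestItem is an interactable world item that completes its associated quest when the player passes a dice roll.
; A capsule overlap shows or hides the interaction prompt, which no longer appears once succeeded.
; Interacting opens WB_DiceRoll behind a DoOnce, which failure resets for retry; success starts and immediately completes the quest through the player's QuestComponent.
; BeginPlay restores completion from saved quest data and listens for quest-completed events.
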(event `self.ReceiveBeginPlay`
  (bind _aswb_interact (cast `/Game/UI/Blueprints/WB_Interact` (`WidgetComponent.GetWidget` (`self.InteractWidget`))))
  (set `/Game/UI/Blueprints/WB_Interact. Text` (`self.InteractionText`) _aswb_interact)
  (bind _asbp_third_person_character (cast `/Game/ThirdPerson/Blueprints/BP_ThirdPersonCharacter` (`GameplayStatics.GetPlayerCharacter` 0)))
  (add `/Game/Quests/QuestComponent.OnQuestCompleted` (`/Game/ThirdPerson/Blueprints/BP_ThirdPersonCharacter.QuestComponent` _asbp_third_person_character) (delegate `OnQuestCompletedEvent`))
  (bind _savegamedata (message `/Game/SaveGame/BPI_SaveGame.GetGameData` (`GameplayStatics.GetGameInstance`)))
  (bind (_playersave_transform _playersave_controlrotation _playersave_currenthealth _playersave_maxhealth _playersave_currentstamina _playersave_maxstamina _playersave_currentxp _playersave_maxxp _playersave_level _playersave_vigor _playersave_endurance _playersave_fitness _playersave_mind _playersave_playerquests) (break `/Game/SaveGame/S_PlayerSave` (`/Game/SaveGame/BP_Save.PlayerSave` _savegamedata)))
  (for _array_element _playersave_playerquests
    (bind (_questid _questname _questdescription _xp _biscompleted) (break `Quest` _array_element))
    (if (== _questid (`self.AssociatedQuestID`))
      (set `self.Succeded` _biscompleted))))

(event `OnQuestCompletedEvent`
  (params (QuestID :type Name))
  (if (== QuestID (`self.AssociatedQuestID`))
    (set `self.Succeded` true)))

(event `self.OnInteract`
  (params (Interactor :type "Actor Object Reference"))
  (`/Engine/EditorBlueprintResources/StandardMacros.DoOnce` false :!label _label
    (:`Completed`
      (bind _returnvalue (`|CreateWidget` "/Game/UI/Blueprints/WB_DiceRoll.WB_DiceRoll_C" null (`self.Roll Struct`)))
      (add `/Game/UI/Blueprints/WB_DiceRoll.FinishedRoll` _returnvalue (delegate `FinishedRoll`))
      (`UserWidget.AddToViewport` _returnvalue 0))))

(event `FinishedRoll`
  (params (Success :type Boolean))
  (if Success
    (set `self.Succeded` true)
    (`self.On Roll Success`)
    (else
      (goto _label :!via `Reset`))))

(event `self.InteractCapsule.OnComponentBeginOverlap`
  (params (OverlappedComponent :type "PrimitiveComponent Object Reference") (OtherActor :type "Actor Object Reference") (OtherComp :type "PrimitiveComponent Object Reference") (OtherBodyIndex :type Integer) (bFromSweep :type Boolean) (SweepResult :type "HitResult Structure (by ref)"))
  (cast `/Game/ThirdPerson/Blueprints/BP_ThirdPersonCharacter` OtherActor)
  (if (not (`self.Succeded`))
    (`SceneComponent.SetVisibility` (`self.InteractWidget`) true false)))

(event `self.InteractCapsule.OnComponentEndOverlap`
  (params (OverlappedComponent :type "PrimitiveComponent Object Reference") (OtherActor :type "Actor Object Reference") (OtherComp :type "PrimitiveComponent Object Reference") (OtherBodyIndex :type Integer))
  (cast `/Game/ThirdPerson/Blueprints/BP_ThirdPersonCharacter` OtherActor)
  (`SceneComponent.SetVisibility` (`self.InteractWidget`) false false))

(fn `On Roll Success`
  (bind _associatedquestid (`self.AssociatedQuestID`))
  (bind _asbp_third_person_character (cast `/Game/ThirdPerson/Blueprints/BP_ThirdPersonCharacter` (`GameplayStatics.GetPlayerCharacter` 0)))
  (bind _questcomponent (`/Game/ThirdPerson/Blueprints/BP_ThirdPersonCharacter.QuestComponent` _asbp_third_person_character))
  (`/Game/Quests/QuestComponent.StartQuest` _questcomponent _associatedquestid)
  (`/Game/Quests/QuestComponent.CompleteQuest` _questcomponent _associatedquestid)
  (`SceneComponent.SetVisibility` (`self.InteractWidget`) false false))

(fn `UserConstructionScript`)