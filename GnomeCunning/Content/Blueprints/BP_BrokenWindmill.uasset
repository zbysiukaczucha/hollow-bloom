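; BP_BrokenWindmill is an interactable windmill that the player repairs by passing a dice-roll check.
; A capsule overlap shows the "Repair" prompt until repaired, and interacting opens a WB_DiceRoll widget behind a DoOnce.
; Success swaps the mesh to rotation materials, starts and immediately completes quest "1" on the player's QuestComponent, and hides the prompt.
; Failure resets the DoOnce, allowing another attempt.
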(event `self.ReceiveBeginPlay`
  (bind _aswb_interact (cast `/Game/UI/Blueprints/WB_Interact` (`WidgetComponent.GetWidget` (`self.InteractWidget`))))
  (set `/Game/UI/Blueprints/WB_Interact. Text` "Repair" _aswb_interact))

(event `self.OnInteract`
  (params (Interactor :type "Actor Object Reference"))
  (`/Engine/EditorBlueprintResources/StandardMacros.DoOnce` false :!label _label
    (:`Completed`
      (bind _returnvalue (`|CreateWidget` "/Game/UI/Blueprints/WB_DiceRoll.WB_DiceRoll_C" null (make `/Game/UI/Roll_Struct` "NewEnumerator2" 15)))
      (add `/Game/UI/Blueprints/WB_DiceRoll.FinishedRoll` _returnvalue (delegate `FinishedRoll`))
      (`UserWidget.AddToViewport` _returnvalue 0))))

(event `FinishedRoll`
  (params (Success :type Boolean))
  (bind _staticmesh (`self.StaticMesh`))
  (if Success
    (`PrimitiveComponent.SetMaterial` _staticmesh 0 "/Game/Medieval_Env/Props/Materials/MI_RotationWood.MI_RotationWood")
    (`PrimitiveComponent.SetMaterial` _staticmesh 1 "/Game/Medieval_Env/Props/Materials/M_Master_Rotation.M_Master_Rotation")
    (bind _asbp_third_person_character (cast `/Game/ThirdPerson/Blueprints/BP_ThirdPersonCharacter` (`GameplayStatics.GetPlayerCharacter` 0)))
    (bind _questcomponent (`/Game/ThirdPerson/Blueprints/BP_ThirdPersonCharacter.QuestComponent` _asbp_third_person_character))
    (`/Game/Quests/QuestComponent.StartQuest` _questcomponent "1")
    (`/Game/Quests/QuestComponent.CompleteQuest` _questcomponent "1")
    (`SceneComponent.SetVisibility` (`self.InteractWidget`) false false)
    (set `self.Succeded` true)
    (else
      (goto _label :!via `Reset`))))

(event `self.InteractCapsule.OnComponentBeginOverlap`
  (params (OverlappedComponent :type "PrimitiveComponent Object Reference") (OtherActor :type "Actor Object Reference") (OtherComp :type "PrimitiveComponent Object Reference") (OtherBodyIndex :type Integer) (bFromSweep :type Boolean) (SweepResult :type "HitResult Structure (by ref)"))
  (cast `/Game/ThirdPerson/Blueprints/BP_ThirdPersonCharacter` OtherActor)
  (if (not (`self.Succeded`))
    (`SceneComponent.SetVisibility` (`self.InteractWidget`) true false)))

(event `self.InteractCapsule.OnComponentEndOverlap`
  (params (OverlappedComponent :type "PrimitiveComponent Object Reference") (OtherActor :type "Actor Object Reference") (OtherComp :type "PrimitiveComponent Object Reference") (OtherBodyIndex :type Integer))
  (cast `/Game/ThirdPerson/Blueprints/BP_ThirdPersonCharacter` OtherActor)
  (`SceneComponent.SetVisibility` (`self.InteractWidget`) false false))

(fn `UserConstructionScript`)