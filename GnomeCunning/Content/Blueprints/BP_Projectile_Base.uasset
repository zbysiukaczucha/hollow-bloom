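; Base projectile Blueprint that flies via ProjectileMovement and ignores its Instigator when moving.
; The construction script applies Speed as initial and max speed, plus Gravity as gravity scale.
; On BeginPlay, a valid HomingTarget enables homing and zeroes the starting velocity.
; A box collision hit fires the OnProjectileImpact dispatcher with the hit result, spawns the impact effect and sound, then destroys the actor.
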(event `self.ReceiveBeginPlay`
  (bind _projectilemovement (`self.ProjectileMovement`))
  (`PrimitiveComponent.IgnoreActorWhenMoving` (`self.BoxCollision`) (`self.Instigator`) true)
  (bind _homing_target (`self.Homing Target`)
    (:`then`
      (set `ProjectileMovementComponent.bIsHomingProjectile` true _projectilemovement)
      (set `ProjectileMovementComponent.HomingTargetComponent` _homing_target _projectilemovement)
      (set `MovementComponent.Velocity` (0.0 0.0 0.0) _projectilemovement))
    (:`else`)))

(event `self.BoxCollision.OnComponentHit`
  (params (HitComponent :type "PrimitiveComponent Object Reference") (OtherActor :type "Actor Object Reference") (OtherComp :type "PrimitiveComponent Object Reference") (NormalImpulse :type "Vector Structure") (Hit :type "HitResult Structure (by ref)"))
  (bind (_bblockinghit _binitialoverlap _time _distance _location) (`GameplayStatics.BreakHitResult` Hit))
  (`self.OnProjectileImpact` Hit)
  (`NiagaraFunctionLibrary.SpawnSystemAtLocation` (`self.ImpactEffect`) _location)
  (`GameplayStatics.PlaySoundAtLocation` (`self.ImpactSound`) _location (struct) 1.0 1.0 0.0 null null null null)
  (`self.K2_DestroyActor`))

(fn `UserConstructionScript`
  (bind _projectilemovement (`self.ProjectileMovement`))
  (bind _output_get (set `ProjectileMovementComponent.InitialSpeed` (`self.Speed`) _projectilemovement))
  (set `ProjectileMovementComponent.MaxSpeed` _output_get _projectilemovement)
  (set `ProjectileMovementComponent.ProjectileGravityScale` (`self.Gravity`) _projectilemovement))