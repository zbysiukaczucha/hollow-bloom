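; Combat component for BP_ThirdPersonCharacter that handles target lock, sword attack combos and directional dodge rolls, with stamina costs on attacks and dodges.
; Target lock sphere-traces from the camera, attaches a marker actor and steers control rotation toward the target each tick.
; Combos continue through montage notifies when attack is pressed again, and a looping timer sphere-traces the sword to apply rate-limited damage.
; Dodge montages follow the pressed key while strafing.
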(event `self.ReceiveBeginPlay`
  ;[1 1 1] Get Player
  (bind _asbp_third_person_character (cast `/Game/ThirdPerson/Blueprints/BP_ThirdPersonCharacter` (`self.GetOwner`)))
  (set `self.PlayerBP` _asbp_third_person_character))

(event `EnhancedInput|/Game/ThirdPerson/Input/Actions/IA_TargetLock`
  (params (ActionValue :type Boolean) (ElapsedSeconds :type "Float (double-precision)") (TriggeredSeconds :type "Float (double-precision)") (InputAction :type "InputAction Object Reference" :default "/Game/ThirdPerson/Input/Actions/IA_TargetLock.IA_TargetLock"))
  (bind _returnvalue (`Actor.GetTransform` (`self.TargetLockActor`)))
  (bind _transformcomponent (`PlayerCameraManager.TransformComponent` (`GameplayStatics.GetPlayerCameraManager` 0)))
  (bind _charactermovement (`Character.CharacterMovement` (`self.PlayerBP`)))
  (bind _charactermovement_2 (`Character.CharacterMovement` (`self.PlayerBP`)))
  (bind (_returnvalue_x _returnvalue_y _returnvalue_z) (`KismetMathLibrary.BreakVector` (`SceneComponent.K2_GetComponentLocation` _transformcomponent)))
  (bind (_returnvalue_roll _returnvalue_pitch _returnvalue_yaw) (`KismetMathLibrary.BreakRotator` (`SceneComponent.K2_GetComponentRotation` _transformcomponent)))
  (bind _returnvalue_2 (`KismetMathLibrary.MakeVector` _returnvalue_x _returnvalue_y (+ _returnvalue_z 20.0)))
  ;[1 1 1] Target Lock
  (:`Started`
    (`self.TargetLockActor`
      (:`then`
        (set `self.TargetLockActor` null)
        (set `CharacterMovementComponent.bOrientRotationToMovement` true _charactermovement_2)
        (set `CharacterMovementComponent.bUseControllerDesiredRotation` false _charactermovement_2)
        (`Actor.K2_DestroyActor` (`self.TargetLockWidget`)))
      (:`else`
        (bind (_outhit _returnvalue_3) (`KismetSystemLibrary.SphereTraceSingleForObjects` :`Start` _returnvalue_2 :`End` (+ _returnvalue_2 (* (`KismetMathLibrary.GetForwardVector` (`KismetMathLibrary.MakeRotator` _returnvalue_roll (+ _returnvalue_pitch 10.0) _returnvalue_yaw)) 2000.0)) :`Radius` 150.0 :`ObjectTypes` (`|MakeArray` "ObjectTypeQuery3" :!type "EObjectTypeQuery Enum") :`DrawTime` 2.0))
        (if _returnvalue_3
          (set `self.TargetLockActor` (`.HitActor` (`GameplayStatics.BreakHitResult` _outhit)))
          (set `CharacterMovementComponent.bOrientRotationToMovement` false _charactermovement)
          (set `CharacterMovementComponent.bUseControllerDesiredRotation` true _charactermovement)
          (bind _returnvalue_4 (`|SpawnActorFromClass` "/Game/Blueprints/BP_TargetLockWidget.BP_TargetLockWidget_C" (`KismetMathLibrary.MakeTransform` (`KismetMathLibrary.MakeVector` (.x (.location _returnvalue)) (.y (.location _returnvalue)) (.z (.location _returnvalue))) (.rotation _returnvalue)) "AlwaysSpawn" "MultiplyWithRoot" null null))
          (bind _output_get (set `self.TargetLockWidget` _returnvalue_4))
          (`Actor.K2_AttachToActor` _output_get (`self.TargetLockActor`) "None" "SnapToTarget" "SnapToTarget" "SnapToTarget" true))))))

(event `self.ReceiveTick`
  (params (DeltaSeconds :type "Float (single-precision)"))
  (bind _playerbp (`self.PlayerBP`))
  (bind (_returnvalue_roll _returnvalue_pitch _returnvalue_yaw) (`KismetMathLibrary.BreakRotator` (`KismetMathLibrary.FindLookAtRotation` (`Actor.K2_GetActorLocation` _playerbp) (`Actor.K2_GetActorLocation` (`self.TargetLockActor`)))))
  ;[1 1 1] Target Lock Update
  (`self.TargetLockActor`
    (:`then`
      (`Controller.SetControlRotation` (`Pawn.GetController` _playerbp) (`KismetMathLibrary.MakeRotator` _returnvalue_roll (- _returnvalue_pitch 20.0) _returnvalue_yaw)))
    (:`else`)))

(event `EnhancedInput|/Game/ThirdPerson/Input/Actions/IA_Attack`
  (params (ActionValue :type Boolean) (ElapsedSeconds :type "Float (double-precision)") (TriggeredSeconds :type "Float (double-precision)") (InputAction :type "InputAction Object Reference" :default "/Game/ThirdPerson/Input/Actions/IA_Attack.IA_Attack"))
  ;[1 1 1] Attack combo
  (:`Started`
    (if (not (`self.IsDodging`))
      (bind _hasenoughstamina (`/Game/Blueprints/BPC_PlayerStats.Decrease Stamina` (`/Game/ThirdPerson/Blueprints/BP_ThirdPersonCharacter.BPC_PlayerStats` (`self.PlayerBP`)) 15.0))
      (if _hasenoughstamina
        (if (not (`self.IsAttacking`))
          (set `self.IsAttacking` true)
          (`|PlayMontage` (`Character.Mesh` (`self.PlayerBP`)) "/Game/Characters/MainCharacter/Animations/MeleeAttack/SwordAttackCombo_Montage.SwordAttackCombo_Montage"
            (:`OnCompleted`
              (set `self.IsAttacking` false :!label _label)
              (set `self.IsComboAttacking` false))
            (:`OnInterrupted`
              (goto _label))
            (:`OnNotifyBegin`
              (if (and (`self.IsAttacking`) (`self.IsComboAttacking`))
                (set `self.IsComboAttacking` false)
                (else
                  (`AnimInstance.Montage_Stop` (`SkeletalMeshComponent.GetAnimInstance` (`Character.Mesh` (`self.PlayerBP`))) 0.2 "/Game/Characters/MainCharacter/Animations/MeleeAttack/SwordAttackCombo_Montage.SwordAttackCombo_Montage")))))
          (else
            (set `self.IsComboAttacking` true)))))))

(event `EndDamageTrace`
  ;[1 1 1] Damage trace
  (if (`KismetSystemLibrary.K2_IsValidTimerHandle` (stale `BeginDamageTrace` _returnvalue))
    (`KismetSystemLibrary.K2_ClearAndInvalidateTimerHandle` (stale `BeginDamageTrace` _returnvalue))))

(event `BeginDamageTrace`
  ;[1 1 1] Damage trace
  (bind _returnvalue (`KismetSystemLibrary.K2_SetTimerDelegate` (delegate `DamageTrace`) 0.01 true)))

(event `DamageTrace`
  (bind _playerbp (`self.PlayerBP`))
  ;[1 1 1] Damage trace
  (bind (_outhit _returnvalue) (`KismetSystemLibrary.SphereTraceSingleForObjects` :`Start` (`SceneComponent.K2_GetComponentLocation` (`/Game/ThirdPerson/Blueprints/BP_ThirdPersonCharacter.Start Sword Trace` _playerbp)) :`End` (`SceneComponent.K2_GetComponentLocation` (`/Game/ThirdPerson/Blueprints/BP_ThirdPersonCharacter.End Sword Trace` _playerbp)) :`Radius` 25.0 :`ObjectTypes` (`|MakeArray` "ObjectTypeQuery3" :!type "EObjectTypeQuery Enum") :`DrawDebugType` "ForOneFrame"))
  (if _returnvalue
    (`/Engine/EditorBlueprintResources/StandardMacros.DoOnce` false :!label _label_2
      (:`Completed`
        (`GameplayStatics.ApplyDamage` (`.HitActor` (`GameplayStatics.BreakHitResult` _outhit)) (`self.Sword Damage`))
        (`KismetSystemLibrary.Delay` 0.3)
        (goto _label_2 :!via `Reset`)))))

(event `EnhancedInput|/Game/ThirdPerson/Input/Actions/IA_Roll`
  (params (ActionValue :type Boolean) (ElapsedSeconds :type "Float (double-precision)") (TriggeredSeconds :type "Float (double-precision)") (InputAction :type "InputAction Object Reference" :default "/Game/ThirdPerson/Input/Actions/IA_Roll.IA_Roll"))
  (bind _playerbp (`self.PlayerBP`))
  (:`Triggered`
    (if (and (`|EnumEquality` (`CharacterMovementComponent.MovementMode` (`Character.CharacterMovement` (`self.PlayerBP`))) "MOVE_Walking") (not (`self.IsDodging`)) (not (`self.IsAttacking`)))
      (bind _hasenoughstamina (`/Game/Blueprints/BPC_PlayerStats.Decrease Stamina` (`/Game/ThirdPerson/Blueprints/BP_ThirdPersonCharacter.BPC_PlayerStats` (`self.PlayerBP`)) 20.0))
      (if _hasenoughstamina
        (`|ExecutionSequence`
          (:`then_0`
            (if (<= (`KismetMathLibrary.VSize` (`Actor.GetVelocity` _playerbp)) 0.0)
              (set `self.MovementDirection` "NewEnumerator2")
              (elif (`CharacterMovementComponent.bUseControllerDesiredRotation` (`Character.CharacterMovement` _playerbp))
                (switch `string` (`KismetTextLibrary.Conv_TextToString` (`KismetInputLibrary.Key_GetDisplayName` (`/Game/ThirdPerson/Blueprints/BP_ThirdPersonCharacter.Direction Key` (`self.PlayerBP`))))
                  (:`W`
                    (set `self.MovementDirection` "NewEnumerator0"))
                  (:`A`
                    (set `self.MovementDirection` "NewEnumerator1"))
                  (:`S`
                    (set `self.MovementDirection` "NewEnumerator2"))
                  (:`D`
                    (set `self.MovementDirection` "NewEnumerator3")))
                (else
                  (set `self.MovementDirection` "NewEnumerator0")))))
          (:`then_1`
            (`|PlayMontage` (`Character.Mesh` (`self.PlayerBP`)) (select `/Game/Blueprints/E_MovementDirection` (`self.MovementDirection`) :`NewEnumerator0` "/Game/Characters/MainCharacter/Animations/Rolling/Dodge_F_Montage.Dodge_F_Montage" :`NewEnumerator1` "/Game/Characters/MainCharacter/Animations/Rolling/Dodge_L_Montage.Dodge_L_Montage" :`NewEnumerator2` "/Game/Characters/MainCharacter/Animations/Rolling/Dodge_B_Montage.Dodge_B_Montage" :`NewEnumerator3` "/Game/Characters/MainCharacter/Animations/Rolling/Dodge_R_Montage.Dodge_R_Montage" :!type "AnimMontage Object Reference")
              (:`then`
                (set `self.IsDodging` true))
              (:`OnBlendOut`
                (set `self.IsDodging` false :!label _label_3))
              (:`OnInterrupted`
                (goto _label_3)))))
        (else
          (goto _label_3))))))