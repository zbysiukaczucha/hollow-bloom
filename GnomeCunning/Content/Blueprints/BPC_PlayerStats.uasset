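; BPC_PlayerStats is an actor component that holds the player's health, stamina, XP, level and four attributes for the third-person character.
; Health and stamina functions apply changes, clamping gains to the maximum, reporting death at zero health and refusing stamina costs the player cannot afford.
; LevelUp derives new maximums from Vigor and Endurance, refills both, carries over surplus XP and refreshes the HUD XP text.
; Reaching the XP threshold does not yet trigger anything.
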(event `self.ReceiveBeginPlay`
  (bind _asbp_third_person_character (cast `/Game/ThirdPerson/Blueprints/BP_ThirdPersonCharacter` (`self.GetOwner`)))
  (set `self.Player Character BP` _asbp_third_person_character))

(fn `Decrease Health`
  (params (Damage :type "Float (double-precision)"))
  (returns (IsPlayerDead :type Boolean))
  (bind _output_get (set `self.Current Health` (- (`self.Current Health`) Damage)))
  (return (<= _output_get 0.0)))

(fn `Decrease Stamina`
  (params (DepletedStamina :type "Float (double-precision)"))
  (returns (HasEnoughStamina :type Boolean))
  (bind _returnvalue (- (`self.Current Stamina`) DepletedStamina))
  (bind _output_get (set `self.HasEnoughStamina` (>= _returnvalue 0.0)))
  (if _output_get
    (set `self.Current Stamina` _returnvalue))
  (return (`self.HasEnoughStamina`)))

(fn `Increase Health`
  (params (AddedHealth :type "Float (double-precision)"))
  (set `self.Current Health` (`KismetMathLibrary.FClamp` (+ AddedHealth (`self.Current Health`)) 0.0 (`self.Max Health`))))

(fn `Increase Stamina`
  (params (AddedStamina :type "Float (double-precision)"))
  (set `self.Current Stamina` (`KismetMathLibrary.FClamp` (+ AddedStamina (`self.Current Stamina`)) 0.0 (`self.Max Stamina`))))

(fn `Increase XP`
  (params (XP :type Integer))
  (set `self.Current XP` (+ XP (`self.Current XP`)))
  (`self.Update XP Text`)
  ;[1 1 1] TODO: If curr xp >= max xp => show level uup button that activates the player isn't fighting
  (if (>= (`self.Current XP`) (`self.Max XP`))
    _))

(fn `Level Up`
  (params (Vigor :type Integer) (Endurance :type Integer) (Fitness :type Integer) (Mind :type Integer))
  (set `self.Vigor` Vigor)
  (set `self.Endurance` Endurance)
  (set `self.Fitness` Fitness)
  (set `self.Mind` Mind)
  ;[1 1 1] Set Max and Current Health
  (bind _output_get (set `self.Max Health` (`KismetMathLibrary.Conv_IntToDouble` (+ (* (`self.Vigor`) 20) 100))))
  (set `self.Current Health` _output_get)
  ;[1 1 1] Set Max and Current Stamina
  (bind _output_get_2 (set `self.Max Stamina` (`KismetMathLibrary.Conv_IntToDouble` (+ (* (`self.Endurance`) 20) 100))))
  (set `self.Current Stamina` _output_get_2)
  ;[1 1 1] Set Max and Current XP
  (set `self.Current XP` (- (`self.Current XP`) (`self.Max XP`)))
  (set `self.Max XP` (+ (`self.Max XP`) 250))
  ;[1 1 1] Increment level
  (`/Engine/EditorBlueprintResources/StandardMacros.IncrementInt` (`self.Level`)
    (:`  `
      (`self.Update XP Text`))))

(fn `Update XP Text`
  (set `TextBlock.Text` (`KismetTextLibrary.Conv_StringToText` (`KismetStringLibrary.Concat_StrStr` (`KismetStringLibrary.Concat_StrStr` (`KismetStringLibrary.Concat_StrStr` (`KismetStringLibrary.Conv_IntToString` (`self.Current XP`)) "/") (`KismetStringLibrary.Conv_IntToString` (`self.Max XP`))) " XP")) (`/Game/UI/WB_HUD.XPText` (`/Game/ThirdPerson/Blueprints/BP_ThirdPersonCharacter.HUD Widget` (`self.Player Character BP`)))))