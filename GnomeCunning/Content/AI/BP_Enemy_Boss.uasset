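; Boss enemy character that swaps the inherited widget component for a full-screen boss health bar added to the viewport on BeginPlay.
; Tick caches weapon trace start and end positions from two boss scene markers.
; Die notifies the AI controller, disables capsule collision, clears the player's target lock and restores movement-oriented rotation.
; After a short delay it removes the health bar and activates the death effect.
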(event `self.ReceiveBeginPlay`
  (`parent.ReceiveBeginPlay`)
  (`ActorComponent.K2_DestroyComponent` (`self.Widget`))
  (bind _returnvalue (`|GenericCreateObject` "/Game/UI/Blueprints/WB_BossHealthbar.WB_BossHealthbar_C"))
  (bind _output_get (set `self.HealthBarWidget` _returnvalue))
  (`UserWidget.AddToViewport` _output_get 0))

(event `self.ReceiveTick`
  (params (DeltaSeconds :type "Float (single-precision)"))
  (set `self.StartTracePosition` (`SceneComponent.K2_GetComponentLocation` (`self.Boss Start Trace`)))
  (set `self.EndTracePosition` (`SceneComponent.K2_GetComponentLocation` (`self.Boss End Trace`))))

(event `/Game/Blueprints/BPI_Damage.Die`
  (bind _asbp_ai_enemy (cast `/Game/AI/BP_AI_Enemy` (`self.GetController`)))
  (`/Game/AI/BP_AI_Enemy.Died` _asbp_ai_enemy)
  (`PrimitiveComponent.SetCollisionEnabled` (`self.CapsuleComponent`) "NoCollision")
  (set `self.IsDead` true)
  (bind _asbp_third_person_character (cast `/Game/ThirdPerson/Blueprints/BP_ThirdPersonCharacter` (`GameplayStatics.GetPlayerCharacter` 0)))
  (bind _combatcomponent (`/Game/ThirdPerson/Blueprints/BP_ThirdPersonCharacter.CombatComponent` _asbp_third_person_character))
  (set `CombatComponent.TargetLockActor` null _combatcomponent)
  (`self.K2_DestroyActor` (`CombatComponent.TargetLockWidget` _combatcomponent))
  (bind _asbp_third_person_character_2 (cast `/Game/ThirdPerson/Blueprints/BP_ThirdPersonCharacter` (`GameplayStatics.GetPlayerCharacter` 0)))
  (bind _charactermovement (`Character.CharacterMovement` _asbp_third_person_character_2))
  (set `CharacterMovementComponent.bOrientRotationToMovement` true _charactermovement)
  (set `CharacterMovementComponent.bUseControllerDesiredRotation` false _charactermovement)
  (`KismetSystemLibrary.Delay` 2.0)
  (`Widget.RemoveFromParent` (`self.HealthBarWidget`))
  (`ActorComponent.SetActive` (`self.DeathEffect`) true false))

(fn `UserConstructionScript`
  (`parent.UserConstructionScript`))