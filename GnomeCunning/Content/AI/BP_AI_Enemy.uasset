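; BP_AI_Enemy is an enemy AI controller that runs a behavior tree when play begins.
; When its PawnSensing component sees a pawn, it sets the IsSeeingTarget flag and stores that pawn as TargetActor on the blackboard.
; Nothing here clears the flag or filters which pawns count as targets.
; A Died event detaches the controlled pawn from the controller, pending destruction.
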(event `self.ReceiveBeginPlay`
  (`self.RunBehaviorTree` (`self.Behavior Tree`)))

(event `self.PawnSensing.OnSeePawn`
  (params (Pawn :type "Pawn Object Reference"))
  (`BlackboardComponent.SetValueAsBool` (`AIBlueprintHelperLibrary.GetBlackboard` null) "IsSeeingTarget" true)
  (`BlackboardComponent.SetValueAsObject` (`AIBlueprintHelperLibrary.GetBlackboard` null) "TargetActor" Pawn))

(event `Died`
  (`Pawn.DetachFromControllerPendingDestroy` (`self.K2_GetPawn`)))

(fn `UserConstructionScript`)