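; BP_Enemy is an enemy with a montage-based sword combo attack that deals melee damage.
; BeginSwordTrace and EndSwordTrace start and clear a fast looping timer that sphere-traces for Pawns between two points on the sword.
; A hit applies SwordDamage through a DoOnce that resets after a short delay, limiting repeat hits.
; Damage the enemy receives is only printed, and the trace draws debug shapes.
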(event `/Game/Blueprints/BPI_Damage.EndSwordTrace`
  ;[1 1 1] Damage trace
  (if (`KismetSystemLibrary.K2_IsValidTimerHandle` (stale `/Game/Blueprints/BPI_Damage.BeginSwordTrace` _returnvalue))
    (`KismetSystemLibrary.K2_ClearAndInvalidateTimerHandle` (stale `/Game/Blueprints/BPI_Damage.BeginSwordTrace` _returnvalue))))

(event `/Game/Blueprints/BPI_Damage.BeginSwordTrace`
  ;[1 1 1] Damage trace
  (bind _returnvalue (`KismetSystemLibrary.K2_SetTimerDelegate` (delegate `DamageTrace`) 0.01 true)))

(event `DamageTrace`
  ;[1 1 1] Damage trace
  (bind (_outhit _returnvalue) (`KismetSystemLibrary.SphereTraceSingleForObjects` :`Start` (`SceneComponent.K2_GetComponentLocation` (`self.Start Sword Trace`)) :`End` (`SceneComponent.K2_GetComponentLocation` (`self.End Sword Trace`)) :`Radius` 25.0 :`ObjectTypes` (`|MakeArray` "ObjectTypeQuery3" :!type "EObjectTypeQuery Enum") :`DrawDebugType` "ForOneFrame"))
  (if _returnvalue
    (`/Engine/EditorBlueprintResources/StandardMacros.DoOnce` false :!label _label
      (:`Completed`
        (`GameplayStatics.ApplyDamage` (`.HitActor` (`GameplayStatics.BreakHitResult` _outhit)) (`self.Sword Damage`))
        (`KismetSystemLibrary.Delay` 0.3)
        (goto _label :!via `Reset`)))))

(event `self.ReceiveAnyDamage`
  (params (Damage :type "Float (single-precision)") (DamageType :type "DamageType Object Reference") (InstigatedBy :type "Controller Object Reference") (DamageCauser :type "Actor Object Reference"))
  (`KismetSystemLibrary.PrintString` (`KismetStringLibrary.Conv_DoubleToString` Damage)))

(fn `SwordAttack`
  (returns (Duration :type "Float (double-precision)"))
  (bind _returnvalue (`self.PlayAnimMontage` "/Game/Characters/MainCharacter/Animations/MeleeAttack/SwordAttackCombo_Montage.SwordAttackCombo_Montage"))
  (return _returnvalue))

(fn `UserConstructionScript`)