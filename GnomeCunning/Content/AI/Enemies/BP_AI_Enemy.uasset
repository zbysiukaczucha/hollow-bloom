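; BP_AI_Enemy is the AI controller for enemy pawns, running a behavior tree and storing the pawn's starting location and rotation.
; Pawn sensing writes the seen pawn to the blackboard as TargetActor and sets IsSeeingTarget, unless the enemy only chases in range and the player is outside it.
; PlayerLeftRange clears the seeing flag, and Died detaches the pawn from the controller pending destroy.
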(event `self.ReceiveBeginPlay`
  (bind _returnvalue (`self.K2_GetPawn`))
  (`self.RunBehaviorTree` (`self.Behavior Tree`))
  (set `self.InitialPosition` (`self.K2_GetActorLocation` _returnvalue))
  (set `self.InitialRotation` (`self.K2_GetActorRotation` _returnvalue)))

(event `self.PawnSensing.OnSeePawn`
  (params (Pawn :type "Pawn Object Reference"))
  (bind _asbp_enemy (cast `/Game/AI/Enemies/BP_Enemy` (`self.K2_GetPawn`)))
  (if (or (`self.PlayerInRange`) (not (`/Game/AI/Enemies/BP_Enemy.ChaseInRangeOnly` _asbp_enemy)))
    (`BlackboardComponent.SetValueAsBool` (`AIBlueprintHelperLibrary.GetBlackboard` null) "IsSeeingTarget" true)
    (`BlackboardComponent.SetValueAsObject` (`AIBlueprintHelperLibrary.GetBlackboard` null) "TargetActor" Pawn)))

(event `Died`
  (`Pawn.DetachFromControllerPendingDestroy` (`self.K2_GetPawn`)))

(event `PlayerLeftRange`
  (`BlackboardComponent.SetValueAsBool` (`AIBlueprintHelperLibrary.GetBlackboard` null) "IsSeeingTarget" false))

(fn `UserConstructionScript`)