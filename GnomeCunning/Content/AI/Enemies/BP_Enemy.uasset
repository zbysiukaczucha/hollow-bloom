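; Enemy character Blueprint with sword and point attacks, a stats-driven healthbar widget and ragdoll death.
; A looping timer sphere-traces along the sword, or between stored positions for bosses, with a DoOnce and delay throttling damage.
; A separate single-point trace deals fixed damage, while functions play normal and strong attack montages.
; When Stats reports death, it drops the physics-simulated sword, notifies BP_AI_Enemy, removes the widget and disables capsule collision.
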(event `self.ReceiveBeginPlay`
  (bind _aswb_enemy_healthbar (cast `/Game/UI/Blueprints/WB_EnemyHealthbar` (`WidgetComponent.GetWidget` (`self.Widget`))))
  (set `/Game/UI/Blueprints/WB_EnemyHealthbar.Stats` (`self.Stats`) _aswb_enemy_healthbar))

(event `/Game/Blueprints/BPI_Damage.EndSwordTrace`
  ;[1 1 1] Damage trace
  (if (`KismetSystemLibrary.K2_IsValidTimerHandle` (stale `/Game/Blueprints/BPI_Damage.BeginSwordTrace` _returnvalue))
    (`KismetSystemLibrary.K2_ClearAndInvalidateTimerHandle` (stale `/Game/Blueprints/BPI_Damage.BeginSwordTrace` _returnvalue))))

(event `/Game/Blueprints/BPI_Damage.BeginSwordTrace`
  ;[1 1 1] Damage trace
  (bind _returnvalue (`KismetSystemLibrary.K2_SetTimerDelegate` (delegate `DamageTrace`) 0.01 true)))

(event `DamageTrace`
  (bind _isboss (`self.IsBoss`))
  ;[1 1 1] Damage trace
  (bind (_outhit _returnvalue) (`KismetSystemLibrary.SphereTraceSingleForObjects` :`Start` (`KismetMathLibrary.SelectVector` (`self.StartTracePosition`) (`SceneComponent.K2_GetComponentLocation` (`self.Start Sword Trace`)) _isboss) :`End` (`KismetMathLibrary.SelectVector` (`self.EndTracePosition`) (`SceneComponent.K2_GetComponentLocation` (`self.End Sword Trace`)) _isboss) :`Radius` (`self.TraceRadius`) :`ObjectTypes` (`|MakeArray` "ObjectTypeQuery3" :!type "EObjectTypeQuery Enum") :`DrawDebugType` "ForOneFrame"))
  (if _returnvalue
    (`/Engine/EditorBlueprintResources/StandardMacros.DoOnce` false :!label _label
      (:`Completed`
        (`GameplayStatics.ApplyDamage` (`.HitActor` (`GameplayStatics.BreakHitResult` _outhit)) (`self.Sword Damage`))
        (`KismetSystemLibrary.Delay` 0.3)
        (goto _label :!via `Reset`)))))

(event `self.ReceiveAnyDamage`
  (params (Damage :type "Float (single-precision)") (DamageType :type "DamageType Object Reference") (InstigatedBy :type "Controller Object Reference") (DamageCauser :type "Actor Object Reference"))
  (bind _returnvalue (`StatsComponent.DecreaseHealth` (`self.Stats`) Damage))
  (if _returnvalue
    (`self.Die`)))

(event `/Game/Blueprints/BPI_Damage.Die`
  (bind _sword (`self.Sword`))
  (`SceneComponent.K2_DetachFromComponent` _sword "KeepWorld" "KeepWorld" "KeepWorld" false)
  (`PrimitiveComponent.SetCollisionEnabled` _sword "QueryAndPhysics")
  (`PrimitiveComponent.SetSimulatePhysics` _sword true)
  (bind _asbp_ai_enemy (cast `/Game/AI/Enemies/BP_AI_Enemy` (`self.GetController`)))
  (`/Game/AI/Enemies/BP_AI_Enemy.Died` _asbp_ai_enemy)
  (`PrimitiveComponent.SetSimulatePhysics` (`self.Mesh`) true)
  (`ActorComponent.K2_DestroyComponent` (`self.Widget`))
  (`PrimitiveComponent.SetCollisionEnabled` (`self.CapsuleComponent`) "NoCollision"))

(event `/Game/Blueprints/BPI_Damage.PointDamageTrace`
  (bind _returnvalue (`SceneComponent.K2_GetComponentLocation` (`self.PointTracePos`)))
  (bind (_outhit _returnvalue_2) (`KismetSystemLibrary.SphereTraceSingleForObjects` :`Start` _returnvalue :`End` _returnvalue :`Radius` (`self.PointAttackRadius`) :`ObjectTypes` (`|MakeArray` "ObjectTypeQuery3" :!type "EObjectTypeQuery Enum") :`DrawDebugType` "ForDuration" :`DrawTime` 1.0))
  (if _returnvalue_2
    (`GameplayStatics.ApplyDamage` (`.HitActor` (`GameplayStatics.BreakHitResult` _outhit)) 30.0)))

(fn `Strong Attack`
  (returns (Duration :type "Float (double-precision)"))
  (bind _returnvalue (`self.PlayAnimMontage` (`self.StrongAttackMontage`)))
  (return _returnvalue))

(fn `SwordAttack`
  (returns (Duration :type "Float (double-precision)"))
  (bind _returnvalue (`self.PlayAnimMontage` (`self.SwordAttackMontage`)))
  (return _returnvalue))

(fn `UserConstructionScript`)