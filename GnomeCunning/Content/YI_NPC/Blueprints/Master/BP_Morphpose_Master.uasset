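; Master NPC Blueprint that adds idle facial life through randomly timed blinks, brow movements and smiles.
; BeginPlay starts three self-restarting loops, each waiting a random delay, then playing a timeline if its Blink, Brow or Mouth flag is set.
; Timeline updates drive named face morph targets on every skeletal mesh component descended from Mesh.
; A separate UpdateIdleAnimation event runs or freezes Mesh animation via play rate, based on the Idle flag.
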(event `Update Idle Animation`
  (`SkeletalMeshComponent.SetPlayRate` (`self.Mesh`) (`KismetMathLibrary.Conv_IntToDouble` (select `bool` (`self.Idle`) :`true` 1))))

(event `self.ReceiveBeginPlay`
  (`|ExecutionSequence`
    (:`then_0`
      ;[0 0 0 1 24] Blink
      (`KismetSystemLibrary.RetriggerableDelay` (`KismetMathLibrary.RandomFloatInRange` 0.5 5.0) :!label _label)
      (if (`self.Blink`)
        (bind (_direction _newtrack_0) (`Timeline|Timeline_Blink` :!via `PlayFromStart`)
          (:`Update`
            (for _array_element (`SceneComponent.GetChildrenComponents` (`self.Mesh`) true)
              (bind _asskeletal_mesh_component (cast `SkeletalMeshComponent` _array_element))
              (`|ExecutionSequence`
                (:`then_0`
                  (`SkeletalMeshComponent.SetMorphTarget` _asskeletal_mesh_component "eyeBlinkLeft" _newtrack_0 true))
                (:`then_1`
                  (`SkeletalMeshComponent.SetMorphTarget` _asskeletal_mesh_component "eyeBlinkRight" _newtrack_0 true)))))
          (:`Finished`
            (goto _label)))
        (else
          (goto _label))))
    (:`then_1`
      ;[0 0 0 1 24] Brow
      (`KismetSystemLibrary.RetriggerableDelay` (`KismetMathLibrary.RandomFloatInRange` 3.0 10.0) :!label _label_2)
      (if (`self.Brow`)
        (bind (_direction_2 _newtrack_0_2) (`Timeline|Timeline_Brow` :!via `PlayFromStart`)
          (:`Update`
            (for _array_element_2 (`SceneComponent.GetChildrenComponents` (`self.Mesh`) true)
              (bind _asskeletal_mesh_component_2 (cast `SkeletalMeshComponent` _array_element_2))
              (`|ExecutionSequence`
                (:`then_0`
                  (`SkeletalMeshComponent.SetMorphTarget` _asskeletal_mesh_component_2 "browDownLeft" _newtrack_0_2 true))
                (:`then_1`
                  (`SkeletalMeshComponent.SetMorphTarget` _asskeletal_mesh_component_2 "browDownRight" _newtrack_0_2 true))
                (:`then_2`
                  (`SkeletalMeshComponent.SetMorphTarget` _asskeletal_mesh_component_2 "browInnerUp" _newtrack_0_2 true)))))
          (:`Finished`
            (goto _label_2)))
        (else
          (goto _label_2))))
    (:`then_2`
      ;[0 0 0 1 24] Smile
      (`KismetSystemLibrary.RetriggerableDelay` (`KismetMathLibrary.RandomFloatInRange` 10.0 25.0) :!label _label_3)
      (if (`self.Mouth`)
        (bind (_direction_3 _newtrack_0_3) (`Timeline|Timeline_Smile` :!via `PlayFromStart`)
          (:`Update`
            (for _array_element_3 (`SceneComponent.GetChildrenComponents` (`self.Mesh`) true)
              (bind _asskeletal_mesh_component_3 (cast `SkeletalMeshComponent` _array_element_3))
              (`|ExecutionSequence`
                (:`then_0`
                  (`SkeletalMeshComponent.SetMorphTarget` _asskeletal_mesh_component_3 "mouthSmileLeft" _newtrack_0_3 true))
                (:`then_1`
                  (`SkeletalMeshComponent.SetMorphTarget` _asskeletal_mesh_component_3 "mouthSmileRight" _newtrack_0_3 true)))))
          (:`Finished`
            (goto _label_3)))
        (else
          (goto _label_3))))))

(fn `UserConstructionScript`)