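; BP_Dice is a die actor that plays a tumbling animation when a roll is triggered.
; A SceneCaptureComponent2D is restricted to render only this actor.
; The roll event bound at BeginPlay starts a fast looping timer that applies a fixed rotation step to the mesh until a counter runs out.
; It then clears the timer, snaps the mesh to zero rotation and resets the counter, without choosing a face.
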(event `self.ReceiveBeginPlay`
  (`SceneCaptureComponent.ShowOnlyActorComponents` (`self.SceneCaptureComponent2D`) self false)
  (add `self.RollDice` (delegate `RollDice_Event`)))

(event `RollDice_Event`
  (bind _returnvalue (`KismetSystemLibrary.K2_SetTimerDelegate` (delegate `Rotating_Event`) 0.01 true))
  (set `self.RotationTimer` _returnvalue))

(event `Rotating_Event`
  (if (> (`self.RotationCounter`) 0)
    (`/Engine/EditorBlueprintResources/StandardMacros.DecrementInt` (`self.RotationCounter`)
      (:`  `
        (`SceneComponent.K2_AddWorldRotation` (`self.StaticMesh`) (struct :`Pitch` -10.0 :`Yaw` 15.0 :`Roll` 25.0) false false)))
    (else
      (`KismetSystemLibrary.K2_ClearAndInvalidateTimerHandle` (`self.RotationTimer`))
      (`SceneComponent.K2_SetWorldRotation` :`self` (`self.StaticMesh`))
      (set `self.RotationCounter` 100))))

(fn `UserConstructionScript`)